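; Ball spawner actor that creates scaled-down Ball actors at the transform of its Arrow component.
; BeginPlay spawns the first ball immediately, while the SpawnBall event waits one second and flips a boolean before spawning.
; When that boolean is true, it calls ChangeVelocityY on the new ball, so successive SpawnBall spawns alternate in whether they get the velocity change.
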(event Custom|SpawnBall
  (bind _arrow (Variables|Default|GetArrow))
  (bind _returnvalue (Transformation|GetWorldTransform _arrow))
  (Utilities|FlowControl|Delay 1.0)
  (bind _output_get (Variables|Default|Setvar (not (Variables|Default|Getvar))))
  (bind _returnvalue_2 (Game|SpawnActorfromClass "/Game/Blueprints/Ball.Ball_C" (Math|Transform|MakeTransform (.location _returnvalue) (.rotation _returnvalue) "0.700000,0.700000,0.700000") "Undefined" 0 0))
  (if _output_get
    (Class|PingPongBall|ChangeVelocityY _returnvalue_2)
    (Variables|Default|Setvar _output_get)))

(event EventBeginPlay
  (bind _arrow (Variables|Default|GetArrow))
  (bind _returnvalue (Transformation|GetWorldTransform _arrow))
  (bind _returnvalue_2 (Game|SpawnActorfromClass "/Game/Blueprints/Ball.Ball_C" (Math|Transform|MakeTransform (.location _returnvalue) (.rotation _returnvalue) "0.700000,0.700000,0.700000") "Undefined" 0 0))
  (if (stale Custom|SpawnBall _output_get)
    (Class|PingPongBall|ChangeVelocityY _returnvalue_2)
    (Variables|Default|Setvar (stale Custom|SpawnBall _output_get))))

(event Collision|EventActorBeginOverlap
  (params (OtherActor :type Actor%20Object%20Reference)))

(event EventTick
  (params (DeltaSeconds :type Float%20%28single-precision%29)))

(fn ConstructionScript)